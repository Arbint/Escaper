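; Boss explosion actor that shatters destructible geometry and then reveals a spinning text, apparently a win message.
; On BeginPlay it applies a very high external cluster strain field with no falloff, sized and centered on its Sphere component.
; After a short delay it unhides the TextRender component, which Tick rotates around yaw at WinRotSpeed.
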(event EventBeginPlay
  (bind _sphere (Variables|Default|GetSphere))
  (Class|FieldSystemComponent|ApplyPhysicsField (Variables|Field|GetFieldSystemComponent) true "Field_ExternalClusterStrain" 0 (Field|SetRadialFalloff (Variables|Default|GetRadialFalloff) 1e+15 0.0 1.0 0.0 (Components|Sphere|GetScaledSphereRadius _sphere) (Transformation|GetWorldLocation _sphere) "Field_FallOff_None"))
  (Utilities|FlowControl|Delay 3.0)
  (Development|SetHiddeninGame (Variables|Default|GetTextRender) false true))

(event EventTick
  (params (DeltaSeconds :type Float%20%28single-precision%29))
  (Transformation|AddRelativeRotation (Variables|Default|GetTextRender) (Math|Rotator|MakeRotator 0.0 0.0 (* DeltaSeconds (Variables|Default|GetWinRotSpeed))) false false))

(fn ConstructionScript)