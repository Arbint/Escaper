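; BP_Door is a two-panel sliding door that opens or closes when its SetDoorOpen event is called.
; Each call plays the door sound at the actor's location, then plays the DoorAnim timeline forward to open or reverses it to close.
; The timeline's OpenAmt interpolates the left and right panels' relative locations from zero to their open offsets, without sweep.
; It has no trigger logic of its own.
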(event EventBeginPlay)

(event Collision|EventActorBeginOverlap
  (params (OtherActor :type Actor%20Object%20Reference)))

(event EventTick
  (params (DeltaSeconds :type Float%20%28single-precision%29)))

(event EventSetDoorOpen
  (params (bIsOpen :type Boolean))
  (Audio|PlaySoundatLocation "/Game/Blueprints/Audio/door_open.door_open" (Transformation|GetActorLocation) "0, 0, 0" 1.0 1.0 0.0 0 0 0 0)
  (if bIsOpen
    (bind _openamt (Timeline|DoorAnim Play)
      (:Update
        (Transformation|SetRelativeLocation (Variables|Default|Getdoor_door_l) (Math|Vector|Lerp(Vector) "0, 0, 0" (Variables|Default|Getl_door_open) _openamt) false false)
        (Transformation|SetRelativeLocation (Variables|Default|Getdoor_door_r) (Math|Vector|Lerp(Vector) "0, 0, 0" (Variables|Default|Getr_door_open) _openamt) false false)))
    (else
      (Timeline|DoorAnim Reverse))))

(fn ConstructionScript)