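; BP_SecCam is a security camera enemy Blueprint that implements the camera's death effects.
; On Die, a sequence starts two timelines: one blinks the reference light in red, the other rotates the pitch pivot toward a fixed roll to make the camera droop.
; The same sequence spawns a Niagara sparkle and an explosion emitter at the pivot's location.
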(event EventBeginPlay)

(event Collision|EventActorBeginOverlap
  (params (OtherActor :type Actor%20Object%20Reference)))

(event EventTick
  (params (DeltaSeconds :type Float%20%28single-precision%29)))

(event EventDie
  (bind _returnvalue (Class|SecurityCamera|GetPitchPivot))
  (bind _returnvalue_2 (Class|SecurityCamera|GetPitchPivot))
  (bind _returnvalue_3 (Transformation|GetWorldLocation _returnvalue))
  (Utilities|FlowControl|Sequence
    (:then_0
      (bind _lightblink (Timeline|DeathLightBlink Play)
        (:Update
          (Rendering|Components|Light|SetLightColor (Class|SecurityCamera|GetRefLight) (* (Math|Color|MakeColor 1.0 0.0 0.0) _lightblink) true))))
    (:then_1
      (bind _fall (Timeline|Fall Play)
        (:Update
          (Transformation|SetRelativeRotation _returnvalue_2 (Math|Rotator|Lerp(Rotator) (Variables|/Script/Engine.SceneComponent|GetRelativeRotation _returnvalue_2) "0, 0,90.000000" _fall) false false))))
    (:then_2
      (Niagara|SpawnSystematLocation "/Game/VFX/NS_Sparkle.NS_Sparkle" _returnvalue_3)
      (Effects|SpawnEmitteratLocation "/Game/VFX/P_Explosion.P_Explosion" _returnvalue_3))))

(fn ConstructionScript)