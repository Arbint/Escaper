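; BP_SecruityCamera is a destructible security camera that sweeps back and forth and has AI sight perception.
; A timeline rotates the yaw pivot across RotationRange, modulating audio volume with the sweep and pausing at each end before a FlipFlop reverses it.
; When health empties, it disables sight, halts the sweep, spawns explosion effects, physics-drops its meshes and animates a red light before destroying itself after a delay.
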(event OnHealthEmpty(Health)
  (bind _returnvalue (Transformation|GetActorLocation))
  (Class|AIPerceptionComponent|SetSenseEnabled (Class|SecruityCamera|GetPerceptionComp) "/Script/AIModule.AISense_Sight" false)
  (Utilities|FlowControl|Sequence
    (:then_0
      (Components|Timeline|SetPlayRate (Variables|Default|GetCamerYaw) 0.0))
    (:then_1
      (Niagara|SpawnSystematLocation "/Game/VFX/NS_Sparkle.NS_Sparkle" _returnvalue)
      (Effects|SpawnEmitteratLocation "/Game/VFX/P_Explosion.P_Explosion" _returnvalue)
      (for _array_element (Actor|GetComponentsByClass "/Script/Engine.StaticMeshComponent")
        (Physics|SetSimulatePhysics _array_element true)
        (Collision|SetCollisionResponsetoChannel _array_element "ECC_GameTraceChannel1" "ECR_Ignore")))
    (:then_2
      (bind _colormult (Timeline|LightBroke Play)
        (:Update
          (Class|SecruityCamera|SetLightColor (* (Utilities|Struct|MakeLinearColor 1.0 0.0 0.0 1.0) _colormult)))))
    (:then_3
      (Utilities|FlowControl|Delay 5.0)
      (Actor|DestroyActor))))

(event EventBeginPlay
  (bind _rotationrange (Variables|Default|GetRotationRange))
  (Components|Timeline|SetPlayRate (Variables|Default|GetCamerYaw) (Variables|Default|GetMoveSpeed))
  (bind _yaw (Timeline|CamerYaw PlayFromStart)
    (:Update
      (Transformation|SetRelativeRotation (Class|SecruityCamera|GetYawPivot) (Math|Rotator|MakeRotator 0.0 0.0 (Math|Float|Lerp _rotationrange (* _rotationrange -1.0) _yaw)) false false)
      (Audio|Components|Audio|SetVolumeMultiplier (Variables|Default|GetAudio) (Math|Float|Clamp(Float) (Math|Trig|Sin(Degrees) (* _yaw 1.8e+02)) 0.0 0.2) :!class /Script/Engine.AudioComponent))
    (:Finished
      (Utilities|FlowControl|Delay (Variables|Default|GetPauseDuration))
      (Utilities|FlowControl|FlipFlop
        (:A
          (Timeline|CamerYaw ReverseFromEnd))
        (:B
          (Timeline|CamerYaw PlayFromStart))))))

(event Collision|EventActorBeginOverlap
  (params (OtherActor :type Actor%20Object%20Reference)))

(event EventTick
  (params (DeltaSeconds :type Float%20%28single-precision%29)))

(event EventStopMoving
  (Components|Timeline|SetPlayRate (Variables|Default|GetCamerYaw) 0.0))

(fn ConstructionScript)